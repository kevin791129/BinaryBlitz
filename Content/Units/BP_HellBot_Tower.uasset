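; Blueprint for the HellBot tower unit, handling its base orientation and attack visual effect.
; On BeginPlay it spawns an inactive Niagara attack emitter attached to the capsule at a fixed offset and picks a random yaw for the base.
; Tick reapplies that yaw in world space, so the base mesh stays fixed regardless of actor rotation.
; Each OnAttackBP event toggles the emitter's active state.
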(event `self.ReceiveBeginPlay`
  (bind _returnvalue (`NiagaraFunctionLibrary.SpawnSystemAttached` "/Game/Units/AttackEmitterSystem.AttackEmitterSystem" (`self.CapsuleComponent`) "None" (500.0 0.0 410.0) (struct) "KeepRelativeOffset" false false))
  (set `self.AttackEffect` _returnvalue)
  (set `self.BaseRotation` (`KismetMathLibrary.MakeRotator` 0.0 0.0 (`KismetMathLibrary.Conv_IntToDouble` (`KismetMathLibrary.RandomInteger` 360)))))

(event `self.ReceiveTick`
  (params (DeltaSeconds :type "Float (single-precision)"))
  (`SceneComponent.K2_SetWorldRotation` (`self.SM_HellBot_Tower_Ranged_base`) (`self.BaseRotation`) false false))

(event `self.OnAttack_BP`
  (`ActorComponent.ToggleActive` (`self.AttackEffect`)))

(fn `UserConstructionScript`)