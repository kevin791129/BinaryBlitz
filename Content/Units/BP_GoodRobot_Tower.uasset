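; BP_GoodRobot_Tower is a robot tower unit Blueprint that handles the attack and death effects and the orientation of its range mesh.
; At BeginPlay it attaches an inactive attack emitter to the capsule at an offset and picks a random yaw.
; Tick holds the range mesh at that world rotation, independent of the actor's own rotation.
; The attack event toggles the emitter, and the death event spawns a scaled-up explosion at the actor's location.
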(event `self.ReceiveBeginPlay`
  (bind _returnvalue (`NiagaraFunctionLibrary.SpawnSystemAttached` "/Game/Units/AttackEmitterSystem.AttackEmitterSystem" (`self.CapsuleComponent`) "None" (750.0 0.0 500.0) (struct) "KeepRelativeOffset" false false))
  (set `self.AttackEffect` _returnvalue)
  (set `self.BaseRotation` (`KismetMathLibrary.MakeRotator` 0.0 0.0 (`KismetMathLibrary.Conv_IntToDouble` (`KismetMathLibrary.RandomInteger` 360)))))

(event `self.ReceiveTick`
  (params (DeltaSeconds :type "Float (single-precision)"))
  (`SceneComponent.K2_SetWorldRotation` (`self.SM_GoodRobot_Tower_Range`) (`self.BaseRotation`) false false))

(event `self.OnAttack_BP`
  (`ActorComponent.ToggleActive` (`self.AttackEffect`)))

(event `self.OnDeath_BP`
  (`NiagaraFunctionLibrary.SpawnSystemAtLocation` "/Game/Assets/VFX/Explotion/Explosion.Explosion" (`self.K2_GetActorLocation`) (struct) (3.0 3.0 3.0)))

(fn `UserConstructionScript`)