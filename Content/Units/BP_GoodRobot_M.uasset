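; BP_GoodRobot_M is a robot unit Blueprint that adds visual effects for attack and death.
; On BeginPlay it attaches two inactive attack emitter systems to the capsule at mirrored left and right forward offsets.
; OnAttackBP toggles both emitters' active state, and OnDeathBP spawns a slightly enlarged explosion at the actor's location.
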(event `self.ReceiveBeginPlay`
  (bind _returnvalue (`NiagaraFunctionLibrary.SpawnSystemAttached` "/Game/Units/AttackEmitterSystem.AttackEmitterSystem" (`self.CapsuleComponent`) "None" (200.0 115.0 85.0) (struct) "KeepRelativeOffset" false false))
  (set `self.AttackEffect_R` _returnvalue)
  (bind _returnvalue_2 (`NiagaraFunctionLibrary.SpawnSystemAttached` "/Game/Units/AttackEmitterSystem.AttackEmitterSystem" (`self.CapsuleComponent`) "None" (200.0 -115.0 80.0) (struct) "KeepRelativeOffset" false false))
  (set `self.AttackEffect_L` _returnvalue_2))

(event `self.OnAttack_BP`
  (`ActorComponent.ToggleActive` (`self.AttackEffect_R`))
  (`ActorComponent.ToggleActive` (`self.AttackEffect_L`)))

(event `self.OnDeath_BP`
  (`NiagaraFunctionLibrary.SpawnSystemAtLocation` "/Game/Assets/VFX/Explotion/Explosion.Explosion" (`self.K2_GetActorLocation`) (struct) (1.2 1.2 1.2)))

(fn `UserConstructionScript`)